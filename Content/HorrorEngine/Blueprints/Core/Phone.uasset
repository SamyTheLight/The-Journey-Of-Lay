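; Horror Engine phone item that, when used while takeable, triggers a one-time cutscene that ends in a return to the menu.
; Use plays a tone, disables player input, plays the SceneIsla level sequence, then opens MenuLevel after a fixed delay.
; AddtoCache and Retake save and restore the item's settings; other use events are empty stubs.
; HiddentText shows a subtitle-shadow widget but is not called here, and template equipment examples are unwired.
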(event `/Game/HorrorEngine/Blueprints/Core/Use.AlternativeUse`
  (params (HorrorEvent :type Boolean))
  ;[1 1 1] Inspection Settings
  (if HorrorEvent
    _))

(event `self.InspectionAlternativeUse`
  ;[1 1 1] Inspection Settings
)

(event `/Game/HorrorEngine/Blueprints/Core/Use.Use`
  (params (HorrorEvent :type Boolean))
  ;[1 1 1] Take Settings
  (if (`self.Takeable`)
    (`/Engine/EditorBlueprintResources/StandardMacros.DoOnce` false
      (:`Completed`
        (`GameplayStatics.PlaySound2D` "/Game/HorrorEngine/Audio/SFX/Phone_Tone3.Phone_Tone3" 1.0 1.0 0.0 null null)
        (`KismetSystemLibrary.Delay` 1.0)
        (`/Game/HorrorEngine/Blueprints/Core/HorrorEngineFunctions.PlayerInput` false)
        (bind _returnvalue (`|CreateWidget` "/Game/HorrorEngine/Blueprints/Widgets/MainHUD.MainHUD_C"))
        (set `Widget.Visibility` "Visible" (`/Game/HorrorEngine/Blueprints/Widgets/MainHUD.UseIcon` _returnvalue))
        (`Widget.SetVisibility` _returnvalue "Hidden")
        (bind (_outactor _returnvalue_2) (`LevelSequencePlayer.CreateLevelSequencePlayer` "/Game/MyContent/Scenes/SceneIsla.SceneIsla"))
        (`MovieSceneSequencePlayer.Play` _returnvalue_2)
        (`KismetSystemLibrary.Delay` 60.0)
        (`GameplayStatics.OpenLevelBySoftObjectPtr` "/Game/HorrorEngine/Maps/MenuLevel.MenuLevel")))))

(event `self.InspectionUse`
  ;[1 1 1] Take Settings
  (if (`self.Takeable`)
    _))

(event `self.InventoryUse`
  ;[1 0.135 0.135] If you want to use it in inventory set here...
)

(event `self.AddToCache`
  ;[1 1 1] AddToSaveCache
  (bind _asmaster (`/Game/HorrorEngine/Blueprints/Core/HorrorEngineFunctions.GetPlayer`))
  (`KismetArrayLibrary.Array_Add` (`/Game/HorrorEngine/Blueprints/Core/HE_SaveGameComponent.InventoryCache` (`/Game/HorrorEngine/HorrorEngine.HE_SaveGameComponent` _asmaster)) (make `/Game/HorrorEngine/Blueprints/Structures/SaveStructures/InventorySave` :`Actor` "NewEnumerator6" :`Mesh Settings` (`self.MeshSettings`) :`InspectionSettings` (`self.InspectionSettings`) :`InventorySettings` (`self.InventorySettings`) :`Custom_MainEquipment` (`self.MainEqipment`))))

(event `self.Retake`
  (params (InventorySave :type "/Game/HorrorEngine/Blueprints/Structures/SaveStructures/InventorySave Structure"))
  (bind ((`MeshSettings_3_F9CB663A436015B590A5528C98BAB95D` _meshsettings) (`InspectionSettings_6_197A27FB439B2AC0AE161CAD69B43F4B` _inspectionsettings) (`InventorySettings_12_F92AC4EA409AB5739DDA0791C58F4309` _inventorysettings) (`Custom_MainEquipment_54_31F757A247929B8B24017BBEB0C9C208` _custom_mainequipment)) (break `/Game/HorrorEngine/Blueprints/Structures/SaveStructures/InventorySave` InventorySave))
  ;[1 1 1] Retake
  (set `self.MeshSettings` _meshsettings)
  (set `self.InspectionSettings` _inspectionsettings)
  (bind _structout (setmembers `/Game/HorrorEngine/Blueprints/Structures/InventorySettings` :`StructRef` _inventorysettings :`Number of Items to Add Inventory` 1))
  (set `self.InventorySettings` _structout)
  (set `self.MainEqipment` _custom_mainequipment)
  (`/Game/HorrorEngine/Blueprints/Core/HorrorEngineFunctions.SetMesh` null (`self.MeshSettings`))
  (`self.SetInspection` (`self.InspectionSettings`))
  (`self.SetInventory` (`self.InventorySettings`))
  (set `self.TakeSound` null)
  (`self.Take` (`self.MainEqipment`) true))

(fn `HiddentText`
  (bind _returnvalue (`|CreateWidget` "/Game/HorrorEngine/Blueprints/Widgets/SubWidgets/DialagShadow.DialagShadow_C"))
  (`Widget.SetVisibility` (`/Game/HorrorEngine/Blueprints/Widgets/SubWidgets/DialagShadow.TextShadowkit` _returnvalue) "Hidden")
  (`Widget.SetVisibility` (`/Game/HorrorEngine/Blueprints/Widgets/SubWidgets/DialagShadow.TextShadowkit2` _returnvalue) "Hidden")
  (`Widget.SetVisibility` (`/Game/HorrorEngine/Blueprints/Widgets/SubWidgets/DialagShadow.TextShadowMa1` _returnvalue) "Hidden")
  (`Widget.SetVisibility` (`/Game/HorrorEngine/Blueprints/Widgets/SubWidgets/DialagShadow.TextShadowMa2` _returnvalue) "Hidden")
  (`Widget.SetVisibility` (`/Game/HorrorEngine/Blueprints/Widgets/SubWidgets/DialagShadow.TextShadowBass` _returnvalue) "Visible")
  (`Widget.SetVisibility` (`/Game/HorrorEngine/Blueprints/Widgets/SubWidgets/DialagShadow.TextShadowBass2` _returnvalue) "Visible")
  (`Widget.SetVisibility` (`/Game/HorrorEngine/Blueprints/Widgets/SubWidgets/DialagShadow.TextShadowHall` _returnvalue) "Hidden")
  (`Widget.SetVisibility` (`/Game/HorrorEngine/Blueprints/Widgets/SubWidgets/DialagShadow.TextShadowHall2` _returnvalue) "Hidden")
  (`UserWidget.AddToViewport` _returnvalue 0))

(fn `UserConstructionScript`
  (`parent.UserConstructionScript`)
  (`/Game/HorrorEngine/Blueprints/Core/HorrorEngineMacros.HM_DefaultConstructions` (`self.CreateNewHorrorEvent`))
  (`self.SetInspection` (`self.InspectionSettings`))
  (`self.SetInventory` (`self.InventorySettings`)))